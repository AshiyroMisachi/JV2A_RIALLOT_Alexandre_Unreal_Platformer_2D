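; Player controller that tracks the player's life and score.
; Life starts at the maximum on BeginPlay, and UpdatePlayerLife applies signed changes, caps the result at the maximum and restarts the level through a console command when it reaches zero or below.
; UpdatePlayerScore adds to the score, and both update functions report to the player only through Print String messages.
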(event EventBeginPlay
  (Variables|Default|SetPlayerLife (Variables|Default|GetPlayerMaxLife)))

(event EventTick
  (params (DeltaSeconds :type Float%20%28single-precision%29)))

(fn ConstructionScript)

(fn UpdatePlayerLife
  (params (Amount :type Integer))
  (if (< Amount 0)
    (Development|PrintString "You lose an hp")
    (else
      (Development|PrintString "You gain an hp")))
  (bind _output_get (Variables|Default|SetPlayerLife (+ (Variables|Default|GetPlayerLife) Amount)))
  (if (> _output_get (Variables|Default|GetPlayerMaxLife))
    (Variables|Default|SetPlayerLife (Variables|Default|GetPlayerMaxLife))
    (elif (<= (Variables|Default|GetPlayerLife) 0)
      (Development|PrintString "You died")
      (Development|ExecuteConsoleCommand (Utilities|String|MakeLiteralString "RestartLevel") 0))))

(fn UpdatePlayerScore
  (params (Amount :type Integer))
  (Variables|Default|SetPlayerScore (+ (Variables|Default|GetPlayerScore) Amount))
  (Development|PrintString "You gain a score point"))